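; BP_Mother is the mother character, which starts a dialogue and has a test for its sitting animations.
; Start creates a WBP_Dialogues widget, cross-links it with the BPCDialogues component, fetches the current row and adds the widget to the viewport.
; TestAnimationMesh plays SittingLookingAround on the mesh, waits for its length, then plays SittingStressed, with debug prints.
; BeginPlay and the construction script are empty.
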(event Custom|Start
  (bind _bpc_dialogues (Variables|Default|GetBPC_Dialogues))
  (bind _returnvalue (UserInterface|CreateWidget "/Game/Game/Blueprints/Widget/WBP_Dialogues.WBP_Dialogues_C"))
  (Variables|/Game/Game/Blueprints/Widget/WBP_Dialogues.WBP_Dialogues_C|SetBPC_Dialogue _returnvalue _bpc_dialogues)
  (Variables|/Game/Game/Blueprints/Components/BPC_Dialogues.BPC_Dialogues_C|SetWBP_Dialogue _bpc_dialogues _returnvalue)
  (Default|GetCurrentRow _bpc_dialogues)
  (UserInterface|Viewport|AddtoViewport _returnvalue 0))

(event Custom|TestAnimationMesh
  (Development|PrintString "Hello")
  (Components|Animation|PlayAnimation (Variables|Character|GetMesh) "/Game/Game/Character/Mother/SittingLookingAround.SittingLookingAround" false)
  (Utilities|FlowControl|Delay (Animation|GetPlayLength (.AnimToPlay (Utilities|Struct|BreakSingleAnimationPlayData (Variables|/Script/Engine.SkeletalMeshComponent|GetAnimationData (Variables|Character|GetMesh))))))
  (Development|PrintString "Hello")
  (Components|Animation|PlayAnimation (Variables|Character|GetMesh) "/Game/Game/Character/Mother/SittingStressed.SittingStressed" false))

(event EventBeginPlay)

(event Collision|EventActorBeginOverlap
  (params (OtherActor :type Actor%20Object%20Reference)))

(event EventTick
  (params (DeltaSeconds :type Float%20%28single-precision%29)))

(fn ConstructionScript)