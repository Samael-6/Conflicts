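; BP_MonsterBrother is the monster brother character, which works with AIC_MonsterBrother to chase the player and flee when flashed.
; On BeginPlay it caches the controller, sets its attack range and registers its own destruction with BP_StrangeDadLetter's end-night event.
; Each tick it switches between walk and faster pursuit speed on player detection, and sends an interact message to whatever a short forward trace hits.
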(event Custom|Destroy
  (Actor|DestroyActor))

(event EventBeginPlay
  (bind _asaic_monster_brother (Utilities|Casting|CastToAIC_MonsterBrother (AI|GetAIController self)))
  (Variables|Default|SetAIC%20Monster%20Brother _asaic_monster_brother)
  (Variables|/Game/Game/Blueprints/Character/Brother/AIC_MonsterBrother.AIC_MonsterBrother_C|SetAttackRange _asaic_monster_brother 1.1e+02)
  (Variables|/Script/Engine.CharacterMovementComponent|SetMaxWalkSpeed (Variables|Character|GetCharacterMovement) 1e+02)
  (bind _returnvalue (Actor|GetActorOfClass "/Game/Game/Blueprints/Actors/BP_StrangeDadLetter.BP_StrangeDadLetter_C"))
  (EventDispatchers|BindEventtoEndNight _returnvalue (delegate Custom|Destroy)))

(event EventTick
  (params (DeltaSeconds :type Float%20%28single-precision%29))
  (bind _startlinetrace (Variables|Default|GetstartlineTrace))
  (bind _returnvalue (Transformation|GetWorldLocation _startlinetrace))
  (bind _outhit (Collision|LineTraceByChannel _returnvalue (+ _returnvalue (* (Math|Vector|GetForwardVector _startlinetrace) 5e+01)) "TraceTypeQuery1" false 0 "None"))
  (Class|BPIInteract|Interact(Message) (.hitactor _outhit))
  (if (Variables|/Game/Game/Blueprints/Character/Brother/AIC_MonsterBrother.AIC_MonsterBrother_C|GetIsPlayerDetected (Variables|Default|GetAIC%20Monster%20Brother))
    (Variables|/Script/Engine.CharacterMovementComponent|SetMaxWalkSpeed (Variables|Character|GetCharacterMovement) 3e+02)
    (else
      (Variables|/Script/Engine.CharacterMovementComponent|SetMaxWalkSpeed (Variables|Character|GetCharacterMovement) 1e+02))))

(event EventGettingFlash
  (Default|Flee (Variables|Default|GetAIC%20Monster%20Brother)))

(fn ConstructionScript)