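; Component that steps through dialogue lines from a data table and shows them on the dialogue widget.
; GetCurrentRow looks up the Dialogues row named by the current index, then UpdateDialogueHUD applies its character name, text and colors to the widget.
; NextRow follows the row's NextRow field to set the index and refresh, so conversation order is defined in the table itself.
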(event EventBeginPlay)

(event EventTick
  (params (DeltaSeconds :type Float%20%28single-precision%29)))

(fn GetCurrentRow
  (bind _returnvalue (Utilities|GetDataTableRow (Variables|Default|GetDialogues) (Utilities|String|StringToName (Utilities|String|ToString(Integer) (Variables|Default|GetIndexDialogue))))
    (:then
      (Variables|Default|SetCurrentRow _returnvalue)
      (CallFunction|UpdateDialogueHUD))))

(fn UpdateDialogueHUD
  (bind _currentrow (Variables|Default|GetCurrentRow))
  (bind _currentrow_2 (Variables|Default|GetCurrentRow))
  (bind (_nextrow _charaname _dialogue) (Utilities|Struct|BreakST_Dialogues _currentrow))
  (bind (_nextrow_2 _charaname_2 _dialogue_2 _namecolor _dialoguecolor) (Utilities|Struct|BreakST_Dialogues _currentrow_2))
  (Appearance|SetColorandOpacity (Variables|/Game/Game/Blueprints/Widget/WBP_Dialogues.WBP_Dialogues_C|GetTB_CharaName (Variables|Default|GetWBP_Dialogue)) _namecolor :!class /Script/UMG.TextBlock)
  (Class|Border|SetBrushColor (Variables|/Game/Game/Blueprints/Widget/WBP_Dialogues.WBP_Dialogues_C|GetLineColorName (Variables|Default|GetWBP_Dialogue)) (.SpecifiedColor (Utilities|Struct|BreakSlateColor _namecolor)))
  (Appearance|SetColorandOpacity (Variables|/Game/Game/Blueprints/Widget/WBP_Dialogues.WBP_Dialogues_C|GetTB_Dialogue (Variables|Default|GetWBP_Dialogue)) _dialoguecolor :!class /Script/UMG.TextBlock)
  (Variables|/Script/UMG.TextBlock|SetText (Variables|/Game/Game/Blueprints/Widget/WBP_Dialogues.WBP_Dialogues_C|GetTB_CharaName (Variables|Default|GetWBP_Dialogue)) _charaname)
  (Variables|/Script/UMG.TextBlock|SetText (Variables|/Game/Game/Blueprints/Widget/WBP_Dialogues.WBP_Dialogues_C|GetTB_Dialogue (Variables|Default|GetWBP_Dialogue)) _dialogue))

(fn NextRow
  (Variables|Default|SetIndexDialogue (.NextRow (Utilities|Struct|BreakST_Dialogues (Variables|Default|GetCurrentRow))))
  (CallFunction|GetCurrentRow))