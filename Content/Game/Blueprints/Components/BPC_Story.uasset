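; BPC_Story is an actor component that steps through a story dialogue stored in the Dialogues data table and shows it on a dialogue widget.
; GetCurrentRow looks up the row named by the current index and writes its text into the TBStory text block.
; NextRow follows each row's NextRow link to load the following line, and returns true once a negative index marks the end.
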(event EventBeginPlay)

(event EventTick
  (params (DeltaSeconds :type Float%20%28single-precision%29)))

(fn GetCurrentRow
  (bind _returnvalue (Utilities|GetDataTableRow (Variables|Default|GetDialogues) (Utilities|String|StringToName (Utilities|String|ToString(Integer) (Variables|Default|GetIndexDialogue))))
    (:then
      (Variables|Default|SetCurrentRow _returnvalue)
      (CallFunction|UpdateDialogueHUD))
    (:RowNotFound
      (Development|PrintString "Y A PAS LA ROW !!!" true true "(R=1.000000,G=0.000000,B=0.000000,A=1.000000)"))))

(fn UpdateDialogueHUD
  (Variables|/Script/UMG.TextBlock|SetText (Variables|/Game/Game/Blueprints/Widget/WBP_StoryTransition.WBP_StoryTransition_C|GetTB_Story (Variables|Default|GetWBP_Dialogue)) (.Dialogue (Utilities|Struct|BreakST_Dialogues (Variables|Default|GetCurrentRow)))))

(fn NextRow
  (bind _output_get (Variables|Default|SetIndexDialogue (.NextRow (Utilities|Struct|BreakST_Dialogues (Variables|Default|GetCurrentRow)))))
  (if (< _output_get 0)
    (return (< _output_get 0))
    (else
      (CallFunction|GetCurrentRow))))