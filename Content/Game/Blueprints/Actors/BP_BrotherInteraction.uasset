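; Trigger actor that stages a one-time scripted encounter with the player's brother.
; On first box overlap it removes player input, plays a fade and fall sound, spawns BP_FrrDay beside the player and opens dialogue through BPCDialogues.
; When the dialogue ends, a second fade with door sounds covers removal of the dialogue UI and brother actor, then input is restored.
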(event OnComponentBeginOverlap(Box)
  (params (OverlappedComponent :type Primitive%20Component%20Object%20Reference) (OtherActor :type Actor%20Object%20Reference) (OtherComp :type Primitive%20Component%20Object%20Reference) (OtherBodyIndex :type Integer) (bFromSweep :type Boolean) (SweepResult :type Hit%20Result%20Structure%20%28by%20ref%29))
  (bind _bpc_dialogues (Variables|Default|GetBPC_Dialogues))
  (Utilities|FlowControl|DoOnce false
    (:Completed
      (bind _asbp_true_player (Utilities|Casting|CastToBP_TruePlayer OtherActor))
      (bind _output_get (Variables|Default|SetBP%20True%20Player _asbp_true_player))
      (Default|RemoveInput _output_get)
      (bind _returnvalue (UserInterface|CreateWidget "/Game/Game/Blueprints/Widget/WBP_Transition.WBP_Transition_C"))
      (UserInterface|Viewport|AddtoViewport _returnvalue 0)
      (UserInterface|Animation|PlayAnimation _returnvalue (Variables|/Game/Game/Blueprints/Widget/WBP_Transition.WBP_Transition_C|GetFadeIn _returnvalue) 0.0 1 "Forward" 0.5 false)
      (Audio|PlaySound2D "/Game/Game/Sons/fallsound.fallsound" 1.0 1.0 0.0 0 0)
      (Utilities|FlowControl|Delay (* (Class|WidgetAnimation|GetEndTime (Variables|/Game/Game/Blueprints/Widget/WBP_Transition.WBP_Transition_C|GetFadeIn _returnvalue)) 3.0))
      (bind _returnvalue_2 (Game|SpawnActorfromClass "/Game/Game/Blueprints/Character/Brother/BP_FrrDay.BP_FrrDay_C" (Math|Transform|MakeTransform (Math|Vector|MakeVector (+ (.x (.location (Transformation|GetActorTransform (Variables|Default|GetBP%20True%20Player)))) 7e+01) (.y (.location (Transformation|GetActorTransform (Variables|Default|GetBP%20True%20Player)))) (.z (.location (Transformation|GetActorTransform (Variables|Default|GetBP%20True%20Player))))) (Math|Rotator|MakeRotator (.roll (.rotation (Transformation|GetActorTransform (Variables|Default|GetBP%20True%20Player)))) (.pitch (.rotation (Transformation|GetActorTransform (Variables|Default|GetBP%20True%20Player)))) 1.8e+02) "1.000000,1.000000,1.000000") "AdjustIfPossibleButAlwaysSpawn" "MultiplyWithRoot" 0 0))
      (Variables|Default|SetBP_Frr _returnvalue_2)
      (UserInterface|Animation|PlayAnimation _returnvalue (Variables|/Game/Game/Blueprints/Widget/WBP_Transition.WBP_Transition_C|GetFadeOut _returnvalue) 0.0 1 "Forward" 1.0 false)
      (Utilities|FlowControl|Delay (Class|WidgetAnimation|GetEndTime (Variables|/Game/Game/Blueprints/Widget/WBP_Transition.WBP_Transition_C|GetFadeOut _returnvalue)))
      (Widget|RemovefromParent _returnvalue)
      (bind _returnvalue_3 (UserInterface|CreateWidget "/Game/Game/Blueprints/Widget/WBP_Dialogues.WBP_Dialogues_C"))
      (Variables|/Game/Game/Blueprints/Widget/WBP_Dialogues.WBP_Dialogues_C|SetBPC_Dialogue _returnvalue_3 _bpc_dialogues)
      (Variables|/Game/Game/Blueprints/Components/BPC_Dialogues.BPC_Dialogues_C|SetWBP_Dialogue _bpc_dialogues _returnvalue_3)
      (Default|GetCurrentRow _bpc_dialogues)
      (UserInterface|Viewport|AddtoViewport _returnvalue_3 0))))

(event Custom|EndEventBrother
  (bind _returnvalue (UserInterface|CreateWidget "/Game/Game/Blueprints/Widget/WBP_Transition.WBP_Transition_C"))
  (UserInterface|Viewport|AddtoViewport _returnvalue 0)
  (UserInterface|Animation|PlayAnimation _returnvalue (Variables|/Game/Game/Blueprints/Widget/WBP_Transition.WBP_Transition_C|GetFadeIn _returnvalue) 0.0 1 "Forward" 0.5 false)
  (Audio|PlaySound2D "/Game/Game/Sons/DoorOpening.DoorOpening" 1.0 1.0 0.0 0 0)
  (Utilities|FlowControl|Delay 2.0)
  (Audio|PlaySound2D "/Game/Game/Sons/DoorClosing.DoorClosing" 1.0 1.0 0.0 0 0)
  (Utilities|FlowControl|Delay (* (Class|WidgetAnimation|GetEndTime (Variables|/Game/Game/Blueprints/Widget/WBP_Transition.WBP_Transition_C|GetFadeIn _returnvalue)) 3.0))
  (Widget|RemovefromParent (Variables|/Game/Game/Blueprints/Components/BPC_Dialogues.BPC_Dialogues_C|GetWBP_Dialogue (Variables|Default|GetBPC_Dialogues)))
  (bind _returnvalue_2 (Actor|GetActorOfClass "/Game/Game/Blueprints/Character/Brother/BP_FrrDay.BP_FrrDay_C"))
  (Actor|DestroyActor _returnvalue_2)
  (UserInterface|Animation|PlayAnimation _returnvalue (Variables|/Game/Game/Blueprints/Widget/WBP_Transition.WBP_Transition_C|GetFadeOut _returnvalue) 0.0 1 "Forward" 1.0 false)
  (Default|AddInput (Variables|Default|GetBP%20True%20Player)))

(event EventBeginPlay
  (EventDispatchers|BindEventtoDialogueEnd (Variables|Default|GetBPC_Dialogues) (delegate Custom|EndEventBrother)))

(fn ConstructionScript)