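; Interactable bed that sends the player to the dream level once the present is open and the homework is done.
; Interact does nothing until the present is open, then either plays a transition fade and loads DreamMap or, if homework is unfinished, briefly shows a bed message widget.
; A DoOnce that resets after the message fades out keeps repeated interactions from stacking messages.
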(event EventBeginPlay)

(event Collision|EventActorBeginOverlap
  (params (OtherActor :type Actor%20Object%20Reference)))

(event EventTick
  (params (DeltaSeconds :type Float%20%28single-precision%29)))

(event EventInteract
  (params (BP_Player :type BP%20True%20Player%20Object%20Reference))
  (if (Variables|/Game/Game/Blueprints/Character/Player/BP_TruePlayer.BP_TruePlayer_C|GetPresentOpen BP_Player)
    (if (Variables|/Game/Game/Blueprints/Character/Player/BP_TruePlayer.BP_TruePlayer_C|GetHomeWorkDid BP_Player)
      (bind _returnvalue (UserInterface|CreateWidget "/Game/Game/Blueprints/Widget/WBP_Transition.WBP_Transition_C"))
      (UserInterface|Viewport|AddtoViewport _returnvalue 0)
      (UserInterface|Animation|PlayAnimation _returnvalue (Variables|/Game/Game/Blueprints/Widget/WBP_Transition.WBP_Transition_C|GetFadeIn _returnvalue) 0.0 1 "Forward" 1.0 false)
      (Utilities|FlowControl|Delay (Class|WidgetAnimation|GetEndTime (Variables|/Game/Game/Blueprints/Widget/WBP_Transition.WBP_Transition_C|GetFadeIn _returnvalue)))
      (Game|OpenLevel(byObjectReference) "/Game/Game/Level/DreamMap.DreamMap")
      (else
        (Utilities|FlowControl|DoOnce false :!label _label
          (:Completed
            (bind _returnvalue_2 (UserInterface|CreateWidget "/Game/Game/Blueprints/Widget/WBP_Messages.WBP_Messages_C"))
            (Default|BedMessage _returnvalue_2)
            (UserInterface|Viewport|AddtoViewport _returnvalue_2 0)
            (UserInterface|Animation|PlayAnimation _returnvalue_2 (Variables|/Game/Game/Blueprints/Widget/WBP_Messages.WBP_Messages_C|GetFadeIn _returnvalue_2) 0.0 1 "Forward" 1.0 false)
            (Utilities|FlowControl|Delay 2.0)
            (UserInterface|Animation|PlayAnimation _returnvalue_2 (Variables|/Game/Game/Blueprints/Widget/WBP_Messages.WBP_Messages_C|GetFadeOut _returnvalue_2) 0.0 1 "Forward" 1.0 false)
            (Utilities|FlowControl|Delay (Class|WidgetAnimation|GetEndTime (Variables|/Game/Game/Blueprints/Widget/WBP_Messages.WBP_Messages_C|GetFadeOut _returnvalue_2)))
            (Widget|RemovefromParent _returnvalue_2)
            (goto _label Reset)))))))

(fn ConstructionScript)