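; Interactable letter actor that shows the player a message from Dad for the current day.
; The first interaction creates WBP_DadsLetter and fills it with the GameInstance's DadsMessages entry indexed by DayNumber.
; A FlipFlop makes the next interaction remove the widget and call CallDestroyGift.
; Ending overlap with the Box does the same whenever the widget reference is valid.
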(event OnComponentEndOverlap(Box)
  (params (OverlappedComponent :type Primitive%20Component%20Object%20Reference) (OtherActor :type Actor%20Object%20Reference) (OtherComp :type Primitive%20Component%20Object%20Reference) (OtherBodyIndex :type Integer))
  (bind _wbp_lettte (Variables|Default|GetWBP_Lettte))
  (Utilities|IsValid _wbp_lettte
    (:Is%20Valid
      (Widget|RemovefromParent _wbp_lettte)
      (Default|CallDestroyGift))))

(event EventBeginPlay)

(event Collision|EventActorBeginOverlap
  (params (OtherActor :type Actor%20Object%20Reference)))

(event EventTick
  (params (DeltaSeconds :type Float%20%28single-precision%29)))

(event EventInteract
  (params (BP_Player :type BP%20True%20Player%20Object%20Reference))
  (bind _gameinstance (Variables|/Game/Game/Blueprints/Character/Player/BP_TruePlayer.BP_TruePlayer_C|GetGameInstance BP_Player))
  (Utilities|FlowControl|FlipFlop
    (:A
      (bind _returnvalue (UserInterface|CreateWidget "/Game/Game/Blueprints/Widget/WBP_DadsLetter.WBP_DadsLetter_C"))
      (bind _output_get (Variables|Default|SetWBP_Lettte _returnvalue))
      (Variables|/Script/UMG.TextBlock|SetText (Variables|/Game/Game/Blueprints/Widget/WBP_DadsLetter.WBP_DadsLetter_C|GetDadsMessage _output_get) (Utilities|Array|Get(acopy) (Variables|/Game/Game/Manager/GI_Conflicts.GI_Conflicts_C|GetDadsMessages _gameinstance) (Variables|/Game/Game/Manager/GI_Conflicts.GI_Conflicts_C|GetDayNumber _gameinstance)))
      (UserInterface|Viewport|AddtoViewport _returnvalue 0))
    (:B
      (Widget|RemovefromParent (Variables|Default|GetWBP_Lettte))
      (Default|CallDestroyGift))))

(fn ConstructionScript)