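; Trigger actor that starts an interaction with BP_Mother when the player enters its box.
; BeginPlay caches the BP_TruePlayer pawn and the BP_Mother found in the level, then resets a DoOnce gate.
; The player's box overlap enters that gate, so only the first one calls Start on the mother and shows the mouse cursor.
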(event OnComponentBeginOverlap(Box)
  (params (OverlappedComponent :type Primitive%20Component%20Object%20Reference) (OtherActor :type Actor%20Object%20Reference) (OtherComp :type Primitive%20Component%20Object%20Reference) (OtherBodyIndex :type Integer) (bFromSweep :type Boolean) (SweepResult :type Hit%20Result%20Structure%20%28by%20ref%29))
  (if (== OtherActor (Variables|Default|GetBP_Player))
    (Utilities|FlowControl|DoOnce false
      (:Completed
        (Default|Start (Variables|Default|GetBP_Mother))
        (Variables|/Script/Engine.PlayerController|SetbShowMouseCursor (Game|GetPlayerController 0) true)))))

(event EventBeginPlay
  (bind _asbp_true_player (Utilities|Casting|CastToBP_TruePlayer (Game|Player|GetPlayerPawn 0)))
  (Variables|Default|SetBP_Player _asbp_true_player)
  (bind _returnvalue (Actor|GetActorOfClass "/Game/Game/Blueprints/Character/BP_Mother.BP_Mother_C"))
  (Variables|Default|SetBP_Mother _returnvalue)
  (Utilities|FlowControl|DoOnce false) ; enters at Reset
)

(fn ConstructionScript)