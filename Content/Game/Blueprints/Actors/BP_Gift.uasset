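; Interactable gift box that plays a one-time opening animation when the player interacts with it.
; The AnimOpenGift timeline adds increments to the parts' relative transforms: TU rises to a height limit, then slides and tilts while the four WC side pieces rotate, spread and lower within limits.
; On BeginPlay it binds to BP_DadLetter, whose event destroys the gift and sets PresentOpen on the stored player.
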(event Custom|DestroySelf
  (Actor|DestroyActor)
  (Variables|/Game/Game/Blueprints/Character/Player/BP_TruePlayer.BP_TruePlayer_C|SetPresentOpen (Variables|Default|GetBP%20Player) true))

(event EventInteract
  (params (BP_Player :type BP%20True%20Player%20Object%20Reference))
  (bind _w_cf (Variables|Default|GetW_CF))
  (bind _w_cl (Variables|Default|GetW_CL))
  (bind _w_cb (Variables|Default|GetW_CB))
  (bind _w_cb_2 (Variables|Default|GetW_CB))
  (bind _w_cl_2 (Variables|Default|GetW_CL))
  (bind _w_cr (Variables|Default|GetW_CR))
  (bind _t_u (Variables|Default|GetT_U))
  (bind _w_cf_2 (Variables|Default|GetW_CF))
  (bind _w_cr_2 (Variables|Default|GetW_CR))
  (bind _w_cb_3 (Variables|Default|GetW_CB))
  (bind _w_cl_3 (Variables|Default|GetW_CL))
  (bind _w_cf_3 (Variables|Default|GetW_CF))
  (bind _t_u_2 (Variables|Default|GetT_U))
  (bind _t_u_3 (Variables|Default|GetT_U))
  (bind _w_cr_3 (Variables|Default|GetW_CR))
  (bind _relativelocation (Variables|/Script/Engine.SceneComponent|GetRelativeLocation _t_u))
  (bind _relativerotation (Variables|/Script/Engine.SceneComponent|GetRelativeRotation _w_cb))
  (bind _relativerotation_2 (Variables|/Script/Engine.SceneComponent|GetRelativeRotation _w_cr_3))
  (bind _relativerotation_3 (Variables|/Script/Engine.SceneComponent|GetRelativeRotation _w_cf))
  (bind _relativerotation_4 (Variables|/Script/Engine.SceneComponent|GetRelativeRotation _w_cl))
  (bind _relativelocation_2 (Variables|/Script/Engine.SceneComponent|GetRelativeLocation _w_cf_2))
  (bind _relativelocation_3 (Variables|/Script/Engine.SceneComponent|GetRelativeLocation _w_cr))
  (bind _relativelocation_4 (Variables|/Script/Engine.SceneComponent|GetRelativeLocation _w_cf_3))
  (bind _relativelocation_5 (Variables|/Script/Engine.SceneComponent|GetRelativeLocation _w_cb_2))
  (bind _relativelocation_6 (Variables|/Script/Engine.SceneComponent|GetRelativeLocation _w_cr_2))
  (bind _relativelocation_7 (Variables|/Script/Engine.SceneComponent|GetRelativeLocation _w_cl_2))
  (bind _relativelocation_8 (Variables|/Script/Engine.SceneComponent|GetRelativeLocation _w_cl_3))
  (bind _relativelocation_9 (Variables|/Script/Engine.SceneComponent|GetRelativeLocation _w_cb_3))
  (bind _relativelocation_10 (Variables|/Script/Engine.SceneComponent|GetRelativeLocation _t_u_2))
  (bind _relativerotation_5 (Variables|/Script/Engine.SceneComponent|GetRelativeRotation _t_u_3))
  (Variables|Default|SetBP%20Player BP_Player)
  (Utilities|FlowControl|DoOnce false
    (:Completed
      (bind _time (Timeline|AnimOpenGift PlayFromStart)
        (:Update
          (if (<= (+ (.z _relativelocation_10) _time) 1.3e+02)
            (Transformation|SetRelativeLocation (Variables|Default|GetT_U) (Math|Vector|MakeVector (.x _relativelocation_10) (.y _relativelocation_10) (+ (.z _relativelocation_10) _time)) false false)
            (else
              (Transformation|SetRelativeLocation (Variables|Default|GetT_U) (Math|Vector|MakeVector (+ _time (.x _relativelocation)) (.y _relativelocation) (.z _relativelocation)) false false)
              (Utilities|FlowControl|Sequence
                (:then_0
                  (Transformation|SetRelativeRotation (Variables|Default|GetT_U) (Math|Rotator|MakeRotator (.roll _relativerotation_5) (+ (.pitch _relativerotation_5) (* _time -1.0)) (.yaw _relativerotation_5)) false false)
                  (if (<= (+ (.roll _relativerotation_2) _time) 1.8e+02)
                    (Transformation|SetRelativeRotation _w_cr_3 (Math|Rotator|MakeRotator (+ (.roll _relativerotation_2) _time) (.pitch _relativerotation_2) (.yaw _relativerotation_2)) false false)
                    (Transformation|SetRelativeRotation _w_cf (Math|Rotator|MakeRotator (+ (.roll _relativerotation_3) _time) (.pitch _relativerotation_3) (.yaw _relativerotation_3)) false false)
                    (Transformation|SetRelativeRotation _w_cl (Math|Rotator|MakeRotator (+ (.roll _relativerotation_4) _time) (.pitch _relativerotation_4) (.yaw _relativerotation_4)) false false)
                    (Transformation|SetRelativeRotation _w_cb (Math|Rotator|MakeRotator (+ (.roll _relativerotation) _time) (.pitch _relativerotation) (.yaw _relativerotation)) false false)))
                (:then_1
                  (if (<= (+ _time (.x _relativelocation_6)) 99.0)
                    (Transformation|SetRelativeLocation _w_cr_2 (Math|Vector|MakeVector (+ _time (.x _relativelocation_6)) (.y _relativelocation_6) (.z _relativelocation_6)) false false)
                    (Transformation|SetRelativeLocation _w_cl_2 (Math|Vector|MakeVector (+ (* _time -1.0) (.x _relativelocation_7)) (.y _relativelocation_7) (.z _relativelocation_7)) false false)
                    (Transformation|SetRelativeLocation _w_cb_2 (Math|Vector|MakeVector (.x _relativelocation_5) (+ (* _time -1.0) (.y _relativelocation_5)) (.z _relativelocation_5)) false false)
                    (Transformation|SetRelativeLocation _w_cf_2 (Math|Vector|MakeVector (.x _relativelocation_2) (+ _time (.y _relativelocation_2)) (.z _relativelocation_2)) false false)))
                (:then_2
                  (if (>= (+ (.z _relativelocation_3) (* _time -1.0)) -0.5)
                    (Transformation|SetRelativeLocation _w_cr (Math|Vector|MakeVector (.x _relativelocation_3) (.y _relativelocation_3) (+ (.z _relativelocation_3) (* _time -1.0))) false false)
                    (Transformation|SetRelativeLocation _w_cl_3 (Math|Vector|MakeVector (.x _relativelocation_8) (.y _relativelocation_8) (+ (.z _relativelocation_8) (* _time -1.0))) false false)
                    (Transformation|SetRelativeLocation _w_cb_3 (Math|Vector|MakeVector (.x _relativelocation_9) (.y _relativelocation_9) (+ (.z _relativelocation_9) (* _time -1.0))) false false)
                    (Transformation|SetRelativeLocation _w_cf_3 (Math|Vector|MakeVector (.x _relativelocation_4) (.y _relativelocation_4) (+ (.z _relativelocation_4) (* _time -1.0))) false false)))))))))))

(event EventBeginPlay
  (bind _returnvalue (Actor|GetActorOfClass "/Game/Game/Blueprints/Actors/BP_DadLetter.BP_DadLetter_C"))
  (EventDispatchers|BindEventtoDestroyGift _returnvalue (delegate Custom|DestroySelf)))

(fn ConstructionScript)