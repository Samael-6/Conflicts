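; BP_LightSwitch is an interactable switch actor that toggles a set of referenced lights on and off.
; On BeginPlay it records the starting intensity of each entry in Lights into the parallel LightIntensity array.
; Interact checks IsOn, then either sets every light to zero intensity or restores each saved value by index.
; IsOn flips inside those loops, so it only changes when Lights has entries.
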(event EventBeginPlay
  (for _array_element (Variables|Default|GetLights)
    (Utilities|Array|Add (Variables|Default|GetLightIntensity) (Variables|/Script/Engine.LightComponentBase|GetIntensity (Variables|/Script/Engine.Light|GetLightComponent _array_element)))))

(event EventInteract
  (params (BP_Player :type BP%20True%20Player%20Object%20Reference))
  (if (Variables|Default|GetIsOn)
    (for _array_element (Variables|Default|GetLights)
      (Rendering|Components|Light|SetIntensity (Variables|/Script/Engine.Light|GetLightComponent _array_element) 0.0)
      (Variables|Default|SetIsOn false))
    (else
      (for (_array_element_2 _array_index) (Variables|Default|GetLights)
        (Rendering|Components|Light|SetIntensity (Variables|/Script/Engine.Light|GetLightComponent _array_element_2) (Utilities|Array|Get(acopy) (Variables|Default|GetLightIntensity) _array_index))
        (Variables|Default|SetIsOn true)))))

(fn ConstructionScript)