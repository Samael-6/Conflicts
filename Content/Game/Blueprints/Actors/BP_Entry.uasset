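; BP_Entry is a trigger actor that starts a dialogue when the player enters its box, once per actor instance.
; The overlap removes player input, links a new WBP_Dialogues widget to the dialogue component and loads the row indexed by GI_Conflicts.RowIndexEntry.
; When the dialogue ends, it restores input, removes the widget and stores the following row index in the game instance for later reads.
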(event OnComponentBeginOverlap(Box)
  (params (OverlappedComponent :type Primitive%20Component%20Object%20Reference) (OtherActor :type Actor%20Object%20Reference) (OtherComp :type Primitive%20Component%20Object%20Reference) (OtherBodyIndex :type Integer) (bFromSweep :type Boolean) (SweepResult :type Hit%20Result%20Structure%20%28by%20ref%29))
  (bind _bpc_dialogues (Variables|Default|GetBPC_Dialogues))
  (if (== OtherActor (Variables|Default|GetBP_Player))
    (Utilities|FlowControl|DoOnce false
      (:Completed
        (Default|RemoveInput (Variables|Default|GetBP_Player))
        (bind _returnvalue (UserInterface|CreateWidget "/Game/Game/Blueprints/Widget/WBP_Dialogues.WBP_Dialogues_C"))
        (Variables|Default|SetWBP_Dialogues _returnvalue)
        (Variables|/Game/Game/Blueprints/Widget/WBP_Dialogues.WBP_Dialogues_C|SetBPC_Dialogue _returnvalue _bpc_dialogues)
        (Variables|/Game/Game/Blueprints/Components/BPC_Dialogues.BPC_Dialogues_C|SetWBP_Dialogue _bpc_dialogues (Variables|Default|GetWBP_Dialogues))
        (Variables|/Game/Game/Blueprints/Components/BPC_Dialogues.BPC_Dialogues_C|SetIndexDialogue _bpc_dialogues (Variables|/Game/Game/Manager/GI_Conflicts.GI_Conflicts_C|GetRowIndexEntry (Variables|Default|GetGameInstance)))
        (Default|GetCurrentRow _bpc_dialogues)
        (UserInterface|Viewport|AddtoViewport (Variables|Default|GetWBP_Dialogues) 0)))))

(event Custom|DialEnded
  (Default|AddInput (Variables|Default|GetBP_Player))
  (Widget|RemovefromParent (Variables|Default|GetWBP_Dialogues))
  (Variables|/Game/Game/Manager/GI_Conflicts.GI_Conflicts_C|SetRowIndexEntry (Variables|Default|GetGameInstance) (+ (Variables|/Game/Game/Blueprints/Components/BPC_Dialogues.BPC_Dialogues_C|GetIndexDialogue (Variables|Default|GetBPC_Dialogues)) 1)))

(event EventBeginPlay
  (bind _asbp_true_player (Utilities|Casting|CastToBP_TruePlayer (Game|Player|GetPlayerPawn 0)))
  (Variables|Default|SetBP_Player _asbp_true_player)
  (bind _asgi_conflicts (Utilities|Casting|CastToGI_Conflicts (Game|GetGameInstance)))
  (Variables|Default|SetGameInstance _asgi_conflicts)
  (EventDispatchers|BindEventtoDialogueEnd (Variables|Default|GetBPC_Dialogues) (delegate Custom|DialEnded)))

(fn ConstructionScript)