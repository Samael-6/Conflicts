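; Interactable door that either swings or shows an on-screen message, depending on InteractionValue.
; A value of 0 creates WBP_DoorMessage, fades it in and out, then removes it, with a DoOnce blocking repeats until it finishes.
; Other values alternate via FlipFlop between reversing and playing a timeline that drives the door's relative yaw, starting with the reverse.
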(event EventInteract
  (params (BP_Player :type BP%20True%20Player%20Object%20Reference))
  (bind _door (Variables|Default|GetDoor))
  (bind _relativerotation (Variables|/Script/Engine.SceneComponent|GetRelativeRotation _door))
  (switch int (Variables|Default|GetInteractionValue)
    (:Default
      (Utilities|FlowControl|FlipFlop
        (:A
          (bind _yaw (Timeline|DoomrTimeline ReverseFromEnd)
            (:Update
              (Transformation|SetRelativeRotation _door (Math|Rotator|MakeRotator (.roll _relativerotation) (.pitch _relativerotation) _yaw) false false))))
        (:B
          (Timeline|DoomrTimeline PlayFromStart))))
    (:0
      (Utilities|FlowControl|DoOnce false :!label _label
        (:Completed
          (bind _returnvalue (UserInterface|CreateWidget "/Game/Game/Blueprints/Widget/WBP_DoorMessage.WBP_DoorMessage_C"))
          (Default|SetMessage _returnvalue)
          (UserInterface|Viewport|AddtoViewport _returnvalue 0)
          (UserInterface|Animation|PlayAnimation _returnvalue (Variables|/Game/Game/Blueprints/Widget/WBP_DoorMessage.WBP_DoorMessage_C|GetFadeIn _returnvalue) 0.0 1 "Forward" 1.0 false)
          (Utilities|FlowControl|Delay (+ (Class|WidgetAnimation|GetEndTime (Variables|/Game/Game/Blueprints/Widget/WBP_DoorMessage.WBP_DoorMessage_C|GetFadeIn _returnvalue)) 1.0))
          (UserInterface|Animation|PlayAnimation _returnvalue (Variables|/Game/Game/Blueprints/Widget/WBP_DoorMessage.WBP_DoorMessage_C|GetFadeOut _returnvalue) 0.0 1 "Forward" 1.0 false)
          (Utilities|FlowControl|Delay (Class|WidgetAnimation|GetEndTime (Variables|/Game/Game/Blueprints/Widget/WBP_DoorMessage.WBP_DoorMessage_C|GetFadeOut _returnvalue)))
          (Widget|RemovefromParent _returnvalue)
          (goto _label Reset))))))

(fn ConstructionScript)