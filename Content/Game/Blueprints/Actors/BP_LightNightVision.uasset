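; BP_LightNightVision is a light actor that changes its rect light when the player switches camera and night vision state.
; On BeginPlay it casts player pawn 0 to BP_TruePlayer and binds SwitchOnOff to that player's camera switch event.
; SwitchOnOff reads IsNightVision, applying the Cam intensity and color when true and the Night pair when false.
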(event Custom|SwitchOnOff
  (bind _rectlight (Variables|Default|GetRectLight))
  (bind _rectlight_2 (Variables|Default|GetRectLight))
  (if (Variables|/Game/Game/Blueprints/Character/Player/BP_TruePlayer.BP_TruePlayer_C|GetIsNightVision (Variables|Default|GetBP_Player))
    (Rendering|Components|Light|SetIntensity _rectlight_2 (Variables|Default|GetIntensityLightCam))
    (Rendering|Components|Light|SetLightColor _rectlight_2 (Variables|Default|GetLightColorCam) true)
    (else
      (Rendering|Components|Light|SetIntensity _rectlight (Variables|Default|GetIntensityLightNight))
      (Rendering|Components|Light|SetLightColor _rectlight (Variables|Default|GetLightColorNight) true))))

(event EventBeginPlay
  (bind _asbp_true_player (Utilities|Casting|CastToBP_TruePlayer (Game|Player|GetPlayerPawn 0)))
  (bind _output_get (Variables|Default|SetBP_Player _asbp_true_player))
  (EventDispatchers|BindEventtoSwitchCamera _output_get (delegate Custom|SwitchOnOff)))

(fn ConstructionScript)